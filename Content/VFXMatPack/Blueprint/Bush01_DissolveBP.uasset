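; Bush dissolve effect Blueprint that drives a material cut on a mesh from the position and orientation of a referenced TargetPoint.
; The construction script creates a dynamic instance of DissolveMaterial on DissolveMesh, sets its emissive dissolve color and applies the initial cut.
; Every Tick updates the material's cut location and direction from the TargetPoint sprite's world location and X axis, so the dissolve follows that actor.
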(event `self.ReceiveTick`
  (params (DeltaSeconds :type "Float (single-precision)"))
  (bind _dissolveinstance (`self.DissolveInstance`))
  (bind _spritecomponent (`TargetPoint.SpriteComponent` (`self.TargetPoint`)))
  ;[1 1 1] RecordCoordinatesTargetPoint
  (`MaterialInstanceDynamic.SetVectorParameterValue` _dissolveinstance (`self.CutLocation`) (`KismetMathLibrary.Conv_VectorToLinearColor` (`SceneComponent.K2_GetComponentLocation` _spritecomponent)))
  (`MaterialInstanceDynamic.SetVectorParameterValue` _dissolveinstance (`self.CutRotate`) (`KismetMathLibrary.Conv_VectorToLinearColor` (`KismetMathLibrary.Conv_RotatorToVector` (`SceneComponent.K2_GetComponentRotation` _spritecomponent)))))

(fn `UserConstructionScript`
  (bind _dissolveinstance (`self.DissolveInstance`))
  (bind _spritecomponent (`TargetPoint.SpriteComponent` (`self.TargetPoint`)))
  ;[1 1 1] SetEmessive
  (bind _returnvalue (`PrimitiveComponent.CreateDynamicMaterialInstance` (`self.DissolveMesh`) 0 (`self.DissolveMaterial`)))
  (set `self.DissolveInstance` _returnvalue)
  (`MaterialInstanceDynamic.SetVectorParameterValue` (`self.DissolveInstance`) (`self.EmessiveDissolve`) (`self.EmessiveDissolveColor`))
  (`MaterialInstanceDynamic.SetVectorParameterValue` _dissolveinstance (`self.CutLocation`) (`KismetMathLibrary.Conv_VectorToLinearColor` (`SceneComponent.K2_GetComponentLocation` _spritecomponent)))
  (`MaterialInstanceDynamic.SetVectorParameterValue` _dissolveinstance (`self.CutRotate`) (`KismetMathLibrary.Conv_VectorToLinearColor` (`KismetMathLibrary.Conv_RotatorToVector` (`SceneComponent.K2_GetComponentRotation` _spritecomponent)))))