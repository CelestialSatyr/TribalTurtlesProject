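; Waterbolt spell projectile that heals the player's Phamos_BP character when it overlaps any actor other than the player.
; Particle spawn, death and collide events on the main system assign templates to separate spawn, death and nuzzle particle components.
; On a hit it calls GainHealth, swaps effects, zeroes projectile velocity and shortens its lifespan.
; The hit applies no damage, only a placeholder comment for it.
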(event `self.ReceiveBeginPlay`
  ;[1 1 1] Set the actor's lifetime
  (`self.SetLifeSpan` 10.0))

(event `self.MainParticleSystem.OnParticleSpawn`
  (params (EventName :type Name) (EmitterTime :type "Float (single-precision)") (Location :type "Vector Structure") (Velocity :type "Vector Structure"))
  ;[1 1 1] Handle all the particles.
  (`ParticleSystemComponent.SetTemplate` (`self.SpawnParticleSystem`) "/Game/InfinityBladeEffects/Effects/FX_Skill_RockBurst/Waterbolt_Begin.Waterbolt_Begin"))

(event `self.MainParticleSystem.OnParticleDeath`
  (params (EventName :type Name) (EmitterTime :type "Float (single-precision)") (ParticleTime :type Integer) (Location :type "Vector Structure") (Velocity :type "Vector Structure") (Direction :type "Vector Structure"))
  ;[1 1 1] Handle all the particles.
  (`ParticleSystemComponent.SetTemplate` (`self.DeathParticleSystem`) "/Game/InfinityBladeEffects/Effects/FX_Combat_Ice/Impact/P_Impact_Ice.P_Impact_Ice"))

(event `self.MainParticleSystem.OnParticleCollide`
  (params (EventName :type Name) (EmitterTime :type "Float (single-precision)") (ParticleTime :type Integer) (Location :type "Vector Structure") (Velocity :type "Vector Structure") (Direction :type "Vector Structure") (Normal :type "Vector Structure") (BoneName :type Name) (PhysMat :type "PhysicalMaterial Object Reference"))
  ;[1 1 1] Handle all the particles.
  (`ParticleSystemComponent.SetTemplate` (`self.NuzzleParticleSystem`) "/Game/InfinityBladeEffects/Effects/FX_Skill_TeleCharge/P_Skill_Telecharge_Ice_Impact_02.P_Skill_Telecharge_Ice_Impact_02"))

(event `self.Collision.OnComponentBeginOverlap`
  (params (OverlappedComponent :type "PrimitiveComponent Object Reference") (OtherActor :type "Actor Object Reference") (OtherComp :type "PrimitiveComponent Object Reference") (OtherBodyIndex :type Integer) (bFromSweep :type Boolean) (SweepResult :type "HitResult Structure (by ref)"))
  ;[1 1 1] Test if spell hit an actor.
  (if (!= OtherActor (`GameplayStatics.GetPlayerCharacter` 0))
    ;[1 1 1] This is where we can do all the effects, such as damage.
    (bind _asphamos_bp (cast `/Game/Characters/Phamos/Phamos_BP` (`GameplayStatics.GetPlayerCharacter` 0)))
    (`/Game/Characters/Phamos/Phamos_BP.GainHealth` _asphamos_bp)
    ;[1 1 1] Handle all the particles.
    (`ParticleSystemComponent.SetTemplate` (`self.DeathParticleSystem`) "/Game/InfinityBladeEffects/Effects/FX_Skill_RockBurst/Waterbolt_Begin.Waterbolt_Begin")
    (`ParticleSystemComponent.SetTemplate` (`self.MainParticleSystem`) null)
    ;[1 1 1] Remove velocity and set the actor's lifespan.
    (`ProjectileMovementComponent.SetVelocityInLocalSpace` (`self.ProjectileMovement`) (0.0 0.0 0.0))
    (`self.SetLifeSpan` 1.5)))

(fn `UserConstructionScript`)