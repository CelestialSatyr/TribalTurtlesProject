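; Fireball spell Blueprint that swaps particle effects and detects contact with test enemies.
; Spawn and death events from the fireball particle system switch the effect's template between power-up and strong-death visuals.
; Collision overlap stores any TestEnemy it meets and prints a hit message, while blocking hits on anything not equal to TestEnemy print a miss.
; Contact responses are debug prints only, with no damage logic.
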(event `self.FireballParticleSystem.OnParticleSpawn`
  (params (EventName :type Name) (EmitterTime :type "Float (single-precision)") (Location :type "Vector Structure") (Velocity :type "Vector Structure"))
  (`ParticleSystemComponent.SetTemplate` (`self.ParticleEffect`) "/Game/InfinityBladeEffects/Effects/FX_Mobile/Fire/combat/P_FireBall_Powerup.P_FireBall_Powerup"))

(event `self.FireballParticleSystem.OnParticleDeath`
  (params (EventName :type Name) (EmitterTime :type "Float (single-precision)") (ParticleTime :type Integer) (Location :type "Vector Structure") (Velocity :type "Vector Structure") (Direction :type "Vector Structure"))
  (`ParticleSystemComponent.SetTemplate` (`self.ParticleEffect`) "/Game/InfinityBladeEffects/Effects/FX_Mobile/Fire/combat/P_FireBall_Strong_Death_01.P_FireBall_Strong_Death_01"))

(event `self.Collision.OnComponentBeginOverlap`
  (params (OverlappedComponent :type "PrimitiveComponent Object Reference") (OtherActor :type "Actor Object Reference") (OtherComp :type "PrimitiveComponent Object Reference") (OtherBodyIndex :type Integer) (bFromSweep :type Boolean) (SweepResult :type "HitResult Structure (by ref)"))
  (bind _astest_enemy (cast `/Game/Characters/Enemies/TestEnemy` OtherActor))
  (set `self.Enemy` OtherActor)
  (if (`KismetArrayLibrary.Array_Contains` (`|MakeArray` _astest_enemy) OtherActor)
    (`KismetSystemLibrary.PrintString` "Hit!")))

(event `self.Collision.OnComponentHit`
  (params (HitComponent :type "PrimitiveComponent Object Reference") (OtherActor :type "Actor Object Reference") (OtherComp :type "PrimitiveComponent Object Reference") (NormalImpulse :type "Vector Structure") (Hit :type "HitResult Structure (by ref)"))
  (if (!= OtherActor "/Game/Characters/Enemies/TestEnemy.TestEnemy")
    (`KismetSystemLibrary.PrintString` "Nope!")))

(fn `UserConstructionScript`)