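; Trigger box that launches the Fhollo_BP character straight up when it overlaps.
; On overlap it overwrites the CharacterMovement velocity with a purely vertical vector, discarding horizontal motion.
; The upward speed is a fixed boost plus the yaw angle of the character's negated velocity, so it varies with the direction of approach.
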(event `self.Box.OnComponentBeginOverlap`
  (params (OverlappedComponent :type "PrimitiveComponent Object Reference") (OtherActor :type "Actor Object Reference") (OtherComp :type "PrimitiveComponent Object Reference") (OtherBodyIndex :type Integer) (bFromSweep :type Boolean) (SweepResult :type "HitResult Structure (by ref)"))
  (bind _fhollo (`self.Fhollo`))
  (bind _asfhollo_bp (cast `/Game/Characters/Fhollo/Fhollo_BP` OtherActor))
  (bind _output_get (set `self.Fhollo` _asfhollo_bp))
  (if (== OtherActor _output_get)
    (set `MovementComponent.Velocity` (+ (`KismetMathLibrary.MakeVector` 0.0 0.0 (+ (`KismetMathLibrary.GetYawPitchFromVector` (.location (`KismetMathLibrary.MakeTransform` (`KismetMathLibrary.NegateVector` (`self.GetVelocity` _fhollo))))) 150.0)) (0.0 0.0 150.0)) (`Character.CharacterMovement` _fhollo))))

(fn `UserConstructionScript`)